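; BP_RouteT is a route actor that wires checkpoint components into a branching path when play begins.
; BeginPlay calls ConnectTo to chain the checkpoints, with a fork at the third one that splits into two two-checkpoint branches.
; It has no other active logic, as the overlap and tick events are disabled and the construction script is empty.
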(event EventBeginPlay
  (Class|CheckPointComponent|Connectto (Variables|Default|GetBP_CheckPointComponent) (Variables|Default|GetBP_CheckPointComponent1))
  (Class|CheckPointComponent|Connectto (Variables|Default|GetBP_CheckPointComponent1) (Variables|Default|GetBP_CheckPointComponent2))
  (Class|CheckPointComponent|Connectto (Variables|Default|GetBP_CheckPointComponent2) (Variables|Default|GetBP_CheckPointComponent3))
  (Class|CheckPointComponent|Connectto (Variables|Default|GetBP_CheckPointComponent3) (Variables|Default|GetBP_CheckPointComponent4))
  (Class|CheckPointComponent|Connectto (Variables|Default|GetBP_CheckPointComponent2) (Variables|Default|GetBP_CheckPointComponent5))
  (Class|CheckPointComponent|Connectto (Variables|Default|GetBP_CheckPointComponent5) (Variables|Default|GetBP_CheckPointComponent6)))

(event Collision|EventActorBeginOverlap
  (params (OtherActor :type Actor%20Object%20Reference)))

(event EventTick
  (params (DeltaSeconds :type Float%20%28single-precision%29)))

(fn ConstructionScript)